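; Highscore save data that keeps an array of score structs, ordered from highest to lowest.
; AddHighscore appends a new entry, re-sorts the array and trims it to at most four entries.
; SortSaveData is a selection sort that repeatedly moves the GetHighscoreValue result into a temporary array.
; GetLowestScoreValue returns the lowest entry and its index but is not called within this graph set.
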(fn GetLowestScoreValue
  (for (_array_element _array_index) (Variables|Default|GetSaveStructs)
    (if (== _array_index 0)
      (LocalVariables|SetLowestScore (.score _array_element))
      (LocalVariables|SetLowestIndex _array_index)
      (elif (< (.score _array_element) (LocalVariables|GetLowestScore))
        (LocalVariables|SetLowestScore (.score _array_element))
        (LocalVariables|SetLowestIndex _array_index))))
  (return (Utilities|Array|Get(acopy) (Variables|Default|GetSaveStructs) (LocalVariables|GetLowestIndex)) (LocalVariables|GetLowestIndex)))

(fn GetHighscoreValue
  (for (_array_element _array_index) (Variables|Default|GetSaveStructs)
    (if (== _array_index 0)
      (LocalVariables|SetHighScore (.score _array_element))
      (LocalVariables|SetHighIndex _array_index)
      (elif (> (.score _array_element) (LocalVariables|GetHighScore))
        (LocalVariables|SetHighScore (.score _array_element))
        (LocalVariables|SetHighIndex _array_index))))
  (return (Utilities|Array|Get(acopy) (Variables|Default|GetSaveStructs) (LocalVariables|GetHighIndex)) (LocalVariables|GetHighIndex)))

(fn SortSaveData
  (while (> (Utilities|Array|Length (Variables|Default|GetSaveStructs)) 0)
    (bind (_highscorestruct _highscoreindex) (CallFunction|GetHighscoreValue))
    (Utilities|Array|Add (LocalVariables|GetTempSaveStructs) _highscorestruct)
    (Utilities|Array|RemoveIndex (Variables|Default|GetSaveStructs) _highscoreindex))
  (Variables|Default|SetSaveStructs (LocalVariables|GetTempSaveStructs)))

(fn AddHighscore
  (params (NewScore :type Highscore%20Struct%20Structure))
  (bind _savestructs (Variables|Default|GetSaveStructs))
  (Utilities|Array|Add (Variables|Default|GetSaveStructs) NewScore)
  (CallFunction|SortSaveData)
  (Utilities|Array|Resize _savestructs (Math|Integer|Min(Integer) 4 (Utilities|Array|Length _savestructs))))