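; Player controller for a pinball game that routes flipper and plunger input to the table's actors and creates the HUD.
; On BeginPlay it finds all flippers, sorting them into left and right lists by flip type, takes the first plunger found, and adds the pinball HUD widget.
; Pressing or releasing a flipper action flips or flops every flipper on that side, while the plunger action charges on press and stops on release.
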(event Custom|DetecFlippers
  (bind _outactors (Actor|GetAllActorsOfClass "/Game/Blueprints/BP_Flipper.BP_Flipper_C"))
  (for _array_element _outactors
    (switch Utilities|FlowControl|Switch|SwitchonFlipType (Variables|/Game/Blueprints/BP_Flipper.BP_Flipper_C|GetFlipType _array_element)
      (:NewEnumerator0
        (Utilities|Array|Add (Variables|Default|GetLeftFlippers) _array_element))
      (:NewEnumerator1
        (Utilities|Array|Add (Variables|Default|GetRightFlippers) _array_element)))))

(event Custom|DetectPlunger
  (bind _outactors (Actor|GetAllActorsOfClass "/Game/Blueprints/BP_Plunger.BP_Plunger_C"))
  (Variables|Default|SetPlunger (Utilities|Array|Get(acopy) _outactors)))

(event Custom|CreatePlayerHUD
  (Viewport|RemoveAllWidgets)
  (bind _returnvalue (UserInterface|CreateWidget "/Game/Blueprints/PinballHUD.PinballHUD_C"))
  (UserInterface|Viewport|AddtoViewport _returnvalue 0))

(event EventBeginPlay
  (CallFunction|DetecFlippers)
  (CallFunction|DetectPlunger)
  (CallFunction|CreatePlayerHUD))

(event EventTick
  (params (DeltaSeconds :type Float%20%28single-precision%29)))

(event Input|ActionEvents|InputActionLeftFlipper
  (params (Key :type Key%20Structure :default "AnyKey"))
  (bind _leftflippers (Variables|Default|GetLeftFlippers))
  (:Pressed
    (for _array_element _leftflippers
      (Default|Flip _array_element)))
  (:Released
    (for _array_element_2 _leftflippers
      (Default|Flop _array_element_2))))

(event Input|ActionEvents|InputActionRightFlipper
  (params (Key :type Key%20Structure :default "AnyKey"))
  (bind _rightflippers (Variables|Default|GetRightFlippers))
  (:Pressed
    (for _array_element _rightflippers
      (Default|Flip _array_element)))
  (:Released
    (for _array_element_2 _rightflippers
      (Default|Flop _array_element_2))))

(event Input|ActionEvents|InputActionPlunger
  (params (Key :type Key%20Structure :default "AnyKey"))
  (bind _plunger (Variables|Default|GetPlunger))
  (:Pressed
    (Default|ChargePlunger _plunger))
  (:Released
    (Default|StopPlunger _plunger)))

(fn ConstructionScript)